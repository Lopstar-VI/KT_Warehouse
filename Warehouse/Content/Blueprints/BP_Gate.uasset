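; BP_Gate is a gate actor that slides open by rising upward when triggered by a loading zone.
; On BeginPlay it stores its start location, computes a raised end location, and binds OpenEvent to the open-door event of BPLoadingZone.
; OpenEvent plays the OpenGate timeline, which lerps the actor between the two locations without sweeping.
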(event Custom|Open%20Event
  ;[0.15 0.15 0.15 0.5] Animation Open Door
  (bind _newtrack_0 (Timeline|Open%20Gate Play)
    (:Update
      (Transformation|SetActorLocation (Math|Vector|Lerp(Vector) (Variables|Default|GetStratLocation) (Variables|Default|GetEndLocation) _newtrack_0) false false))))

(event EventBeginPlay
  ;[0.15 0.15 0.15 0.5] Save Location Vector
  (bind _output_get (Variables|Default|SetStratLocation (Transformation|GetActorLocation)))
  (Variables|Default|SetEndLocation (+ _output_get "0.000000,0.000000,100.000000"))
  (EventDispatchers|BindEventtoOpenDoor (Variables|Default|GetBP_Loading%20Zone) (delegate Custom|Open%20Event)))

(fn ConstructionScript)