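; BP_LoadingZone is a delivery zone that counts boxes placed on its pallet and triggers a door opening once three have arrived.
; An overlap on the pallet collision accepts only BP_Box actors and flags each as delivered, so none counts twice.
; Each new delivery prints progress to the screen, and the third calls OpenDoor.
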(event OnComponentBeginOverlap(Pallet_collision)
  (params (OverlappedComponent :type Primitive%20Component%20Object%20Reference) (OtherActor :type Actor%20Object%20Reference) (OtherComp :type Primitive%20Component%20Object%20Reference) (OtherBodyIndex :type Integer) (bFromSweep :type Boolean) (SweepResult :type Hit%20Result%20Structure%20%28by%20ref%29))
  (bind _asbp_box (Utilities|Casting|CastToBP_Box OtherActor))
  (if (not (Variables|/Game/Blueprints/BP_Box.BP_Box_C|GetIs%20deliverd _asbp_box))
    (Variables|/Game/Blueprints/BP_Box.BP_Box_C|SetIs%20deliverd _asbp_box true)
    (Variables|Default|SetBox%20deliverd (+ (Variables|Default|GetBox%20deliverd) 1))
    (CallFunction|PrintProgress)
    (if (== (Variables|Default|GetBox%20deliverd) 3)
      (Default|CallOpenDoor))))

(event EventBeginPlay)

(event Collision|EventActorBeginOverlap
  (params (OtherActor :type Actor%20Object%20Reference)))

(event EventTick
  (params (DeltaSeconds :type Float%20%28single-precision%29)))

(fn ConstructionScript)

(fn PrintProgress
  (Development|PrintString (Utilities|String|ToString(Text) (Utilities|Text|FormatText "Collected Box: {CurBox} / 3" (Variables|Default|GetBox%20deliverd))) true true "(R=0.007741,G=1.000000,B=0.061176,A=1.000000)"))